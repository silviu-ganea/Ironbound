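; AI controller that drives SandboxCharacter_Mover fighters to attack opponents on other teams.
; A looping 0.1-second timer started on BeginPlay runs the engagement loop, skipping team 0 pawns and those dead or committed to a combat execution.
; The loop scans all fighters for the nearest living enemy on a non-zero team, calls AttemptAttack on it and stops movement when that succeeds.
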(event Custom|DoAttack
  (CallFunction|RunEngagementLoop))

(event EventTick
  (params (DeltaSeconds :type Float%20%28single-precision%29)))

(event EventBeginPlay
  (Utilities|Casting|CastToSandboxCharacter_Mover (Pawn|GetControlledPawn))
  (Utilities|Time|SetTimerbyEvent (delegate Custom|DoAttack) 0.1 true false 1.0))

(fn ConstructionScript)

(fn RunEngagementLoop
  (bind _assandbox_character_mover (Utilities|Casting|CastToSandboxCharacter_Mover (Pawn|GetControlledPawn)))
  (LocalVariables|SetSelf _assandbox_character_mover)
  (if (not (== (Variables|/Game/Blueprints/SandboxCharacter_Mover.SandboxCharacter_Mover_C|GetFighterTeam _assandbox_character_mover) 0))
    (if (not (or (Variables|/Game/Blueprints/SandboxCharacter_Mover.SandboxCharacter_Mover_C|GetIsDead _assandbox_character_mover) (Class|IronboundCombatExecutionComponent|IsCommitted (Variables|/Game/Blueprints/SandboxCharacter_Mover.SandboxCharacter_Mover_C|GetCombatExecution _assandbox_character_mover))))
      (bind _outactors (Actor|GetAllActorsOfClass "/Game/Blueprints/SandboxCharacter_Mover.SandboxCharacter_Mover_C"))
      (Variables|Default|SetAllFighters _outactors)
      (for _array_element (Variables|Default|GetAllFighters)
        (if (and (and (!= _array_element _assandbox_character_mover) (!= (Variables|/Game/Blueprints/SandboxCharacter_Mover.SandboxCharacter_Mover_C|GetFighterTeam _array_element) (Variables|/Game/Blueprints/SandboxCharacter_Mover.SandboxCharacter_Mover_C|GetFighterTeam _assandbox_character_mover))) (and (!= (Variables|/Game/Blueprints/SandboxCharacter_Mover.SandboxCharacter_Mover_C|GetFighterTeam _array_element) 0) (not (Variables|/Game/Blueprints/SandboxCharacter_Mover.SandboxCharacter_Mover_C|GetIsDead _array_element))))
          (LocalVariables|SetLoopDistance (Transformation|GetDistanceTo _assandbox_character_mover _array_element))
          (if (or (not (Utilities|IsValid (LocalVariables|GetBestTarget))) (< (Transformation|GetDistanceTo _assandbox_character_mover _array_element) (LocalVariables|GetBestDistance)))
            (LocalVariables|SetBestTarget _array_element)
            (LocalVariables|SetBestDistance (Transformation|GetDistanceTo _assandbox_character_mover _array_element)))))
      (if (not (not (Utilities|IsValid (LocalVariables|GetBestTarget))))
        (bind _bcommitted (Default|AttemptAttack _assandbox_character_mover (LocalVariables|GetBestTarget)))
        (if _bcommitted
          (AI|Navigation|StopMovement))))))