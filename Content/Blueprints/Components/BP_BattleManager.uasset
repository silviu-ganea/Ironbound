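; Battle manager actor that keeps track of which pawns fight on which team.
; RegisterFighter searches the Teams array for the given TeamId and adds the pawn uniquely to that team's fighters, or appends a new team when none matches.
; When updating an existing team, the rewritten struct takes the AddUnique return value as its TeamId instead of the original ID.
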(event EventBeginPlay)

(event Collision|EventActorBeginOverlap
  (params (OtherActor :type Actor%20Object%20Reference)))

(event EventTick
  (params (DeltaSeconds :type Float%20%28single-precision%29)))

(fn ConstructionScript)

(fn RegisterFighter
  (params (Pawn :type Actor%20Object%20Reference) (TeamId :type Integer))
  (Variables|Default|SetFoundTeam false)
  (for (_array_element _array_index) (Variables|Default|GetTeams)
    (if (== (.TeamId (Utilities|Struct|BreakS_BattleTeam _array_element)) TeamId)
      (Variables|Default|SetFoundTeam true)
      (bind _output_get (Variables|Default|SetUpdatedFighters (.Fighters (Utilities|Struct|BreakS_BattleTeam _array_element))))
      (bind _returnvalue (Utilities|Array|AddUnique (Variables|Default|GetUpdatedFighters) Pawn))
      (Utilities|Array|SetArrayElem (Variables|Default|GetTeams) _array_index (Utilities|Struct|MakeS_BattleTeam _returnvalue _output_get))))
  (if (not (Variables|Default|GetFoundTeam))
    (Utilities|Array|AddUnique (Variables|Default|GetTeams) (Utilities|Struct|MakeS_BattleTeam TeamId (Utilities|Array|MakeArray Pawn)))))