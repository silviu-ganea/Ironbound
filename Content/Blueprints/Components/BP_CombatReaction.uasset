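; Actor component that receives combat hits for a fighter and passes valid ones on as damage.
; On BeginPlay it caches the owner's BP_FighterVitals component.
; ReceiveCombatHit applies the damage to Vitals only when the owner's Team is above zero and differs from the attacker's team, which blocks friendly fire.
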(event EventBeginPlay
  (Variables|Default|SetVitals (Actor|GetComponentbyClass (Components|GetOwner) "/Game/Blueprints/Components/BP_FighterVitals.BP_FighterVitals_C")))

(event EventTick
  (params (DeltaSeconds :type Float%20%28single-precision%29)))

(fn ReceiveCombatHit
  (params (DamageAmount :type Float%20%28double-precision%29) (AttackerTeam :type Float%20%28double-precision%29))
  (if (and (> (Variables|Default|GetTeam) 0) (!= AttackerTeam (Variables|Default|GetTeam)))
    (Default|TakeDamage (Variables|Default|GetVitals) DamageAmount)))